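; Base character Blueprint for a GGJ game that connects health and mana to the on-screen HUD.
; BeginPlay adds crosshair and HUD widgets to the viewport, fills in both readouts from GGJHealth and GGJMana, then binds UsePower to OnUsePower.
; Updates are event-driven: AnyDamage refreshes health and UsePower refreshes mana, each reading current and default values once the HUD reference is validated.
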(event `self.ReceiveAnyDamage`
  (params (Damage :type "Float (single-precision)") (DamageType :type "DamageType Object Reference") (InstigatedBy :type "Controller Object Reference") (DamageCauser :type "Actor Object Reference"))
  (bind _hud_ref (`self.HUD_Ref`))
  (bind _ggj_health (`self.GGJ_Health`))
  (`/Engine/EditorBlueprintResources/StandardMacros.IsValid` _hud_ref
    (:`Is Valid`
      (`/Game/Blueprints/Widgets/WBP_HUD.UpdateHealth` _hud_ref (`GGJ_HealthComponent.CurrentHealth` _ggj_health) (`GGJ_HealthComponent.DefaultHealth` _ggj_health)))))

(event `self.ReceiveBeginPlay`
  (bind _ggj_health (`self.GGJ_Health`))
  (bind _ggj_mana (`self.GGJ_Mana`))
  (`|ExecutionSequence`
    (:`then_0`
      (bind _returnvalue (`|CreateWidget` "/Game/Blueprints/Widgets/WBP_Crosshair.WBP_Crosshair_C"))
      (`UserWidget.AddToViewport` _returnvalue 0)
      (bind _returnvalue_2 (`|CreateWidget` "/Game/Blueprints/Widgets/WBP_HUD.WBP_HUD_C"))
      (bind _output_get (set `self.HUD_Ref` _returnvalue_2))
      (`UserWidget.AddToViewport` _output_get 0)
      (`/Game/Blueprints/Widgets/WBP_HUD.UpdateHealth` _output_get (`GGJ_HealthComponent.CurrentHealth` _ggj_health) (`GGJ_HealthComponent.DefaultHealth` _ggj_health))
      (`/Game/Blueprints/Widgets/WBP_HUD.UpdateMana` _output_get (`GGJ_ManaComponent.CurrentMana` _ggj_mana) (`GGJ_ManaComponent.DefaultMana` _ggj_mana)))
    (:`then_1`
      (add `self.OnUsePower` (delegate `UsePower`)))))

(event `UsePower` :!signature `self.OnUsePower`
  (params (ManaCost :type "Float (double-precision)"))
  (bind _hud_ref (`self.HUD_Ref`))
  (bind _ggj_mana (`self.GGJ_Mana`))
  (`/Engine/EditorBlueprintResources/StandardMacros.IsValid` _hud_ref
    (:`Is Valid`
      (`/Game/Blueprints/Widgets/WBP_HUD.UpdateMana` _hud_ref (`GGJ_ManaComponent.CurrentMana` _ggj_mana) (`GGJ_ManaComponent.DefaultMana` _ggj_mana)))))

(fn `UserConstructionScript`)